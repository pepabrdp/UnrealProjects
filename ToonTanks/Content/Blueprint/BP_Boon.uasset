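; BP_Boon is a Toon Tanks pickup that opens a boon selection screen when the player overlaps its collision box.
; On overlap it creates WBP_BoonSelection, shows the cursor, switches to UI-only input and pauses the game.
; It draws three random indices from BP_GameModeToonTanks, passing earlier picks into later draws, then fills each option with name and gear cost.
; The actor then destroys itself.
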(event OnComponentBeginOverlap(CollisionBox)
  (params (OverlappedComponent :type Primitive%20Component%20Object%20Reference) (OtherActor :type Actor%20Object%20Reference) (OtherComp :type Primitive%20Component%20Object%20Reference) (OtherBodyIndex :type Integer) (bFromSweep :type Boolean) (SweepResult :type Hit%20Result%20Structure%20%28by%20ref%29))
  (bind _returnvalue (Game|GetPlayerController 0))
  (bind _isplayer (Class|BPIPlayer|IsPlayer?(Message) OtherActor))
  (if _isplayer
    ;[1 1 1] If Player, Spawn Widget for boon selection
    (bind _returnvalue_2 (UserInterface|CreateWidget "/Game/Blueprint/Widgets/WBP_BoonSelection.WBP_BoonSelection_C"))
    (Variables|Default|SetBoonSelectionWidget _returnvalue_2)
    (UserInterface|Viewport|AddtoViewport _returnvalue_2 0)
    (Variables|/Script/Engine.PlayerController|SetbShowMouseCursor _returnvalue true)
    (Input|SetInputModeUIOnly _returnvalue 0 "DoNotLock" true)
    (Game|SetGamePaused true)
    ;[1 1 1] Boon Option1
    (bind _asbp_game_mode_toon_tanks (Utilities|Casting|CastToBP_GameModeToonTanks (Game|GetGameMode)))
    (bind _returnvalue_3 (Class|GameModeToonTanks|GetFirstRandomIndex _asbp_game_mode_toon_tanks))
    (Variables|Default|SetFirstRandomIndex _returnvalue_3)
    (bind _returnvalue_4 (Class|GameModeToonTanks|ReturnfromIndex _asbp_game_mode_toon_tanks (Variables|Default|GetFirstRandomIndex)))
    (bind _returnvalue_5 (Class|GameModeToonTanks|ReturnBoonCost _asbp_game_mode_toon_tanks _returnvalue_4))
    (Default|SetBoonOption (Variables|Default|GetBoonSelectionWidget) (Variables|Default|GetFirstRandomIndex) (Utilities|String|ToString(Name) _returnvalue_4) 1 _returnvalue_5)
    ;[1 1 1] Boon Option2
    (bind _returnvalue_6 (Class|GameModeToonTanks|GetSecondRandomIndex _asbp_game_mode_toon_tanks (Variables|Default|GetFirstRandomIndex)))
    (Variables|Default|SetSecondRandomIndex _returnvalue_6)
    (bind _returnvalue_7 (Class|GameModeToonTanks|ReturnfromIndex _asbp_game_mode_toon_tanks (Variables|Default|GetSecondRandomIndex)))
    (bind _returnvalue_8 (Class|GameModeToonTanks|ReturnBoonCost _asbp_game_mode_toon_tanks _returnvalue_7))
    (Default|SetBoonOption (Variables|Default|GetBoonSelectionWidget) (Variables|Default|GetSecondRandomIndex) (Utilities|String|ToString(Name) _returnvalue_7) 2 _returnvalue_8)
    ;[1 1 1] Boon Option3
    (bind _returnvalue_9 (Class|GameModeToonTanks|GetThirdRandomIndex _asbp_game_mode_toon_tanks (Variables|Default|GetFirstRandomIndex) (Variables|Default|GetSecondRandomIndex)))
    (Variables|Default|SetThirdRandomIndex _returnvalue_9)
    (bind _returnvalue_10 (Class|GameModeToonTanks|ReturnfromIndex _asbp_game_mode_toon_tanks (Variables|Default|GetThirdRandomIndex)))
    (bind _returnvalue_11 (Class|GameModeToonTanks|ReturnBoonCost _asbp_game_mode_toon_tanks _returnvalue_10))
    (Default|SetBoonOption (Variables|Default|GetBoonSelectionWidget) (Variables|Default|GetThirdRandomIndex) (Utilities|String|ToString(Name) _returnvalue_10) 3 _returnvalue_11)
    (Actor|DestroyActor)))

(event EventBeginPlay)

(event Collision|EventActorBeginOverlap
  (params (OtherActor :type Actor%20Object%20Reference)))

(event EventTick
  (params (DeltaSeconds :type Float%20%28single-precision%29)))

(fn ConstructionScript)