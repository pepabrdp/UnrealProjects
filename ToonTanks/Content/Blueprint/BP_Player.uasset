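; Player pawn with a base and turret mesh, providing unlockable rewards and revival on top of a Health component.
; Unlock events spawn a party hat at its spawn point and attach it to the turret, or raise health and max health.
; Revive plays a sound, waits briefly, unhides the actor, re-enables tick, fully heals and calls ResurrectingbAlive.
; A debug P key spawns a trail effect at the base mesh, and IsPlayer? reports whether the pawn is controlled.
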(event EventBeginPlay)

(event Collision|EventActorBeginOverlap
  (params (OtherActor :type Actor%20Object%20Reference)))

(event EventTick
  (params (DeltaSeconds :type Float%20%28single-precision%29)))

(event EventUnlockPartyHat
  (bind _returnvalue (Game|SpawnActorfromClass "/Game/Blueprint/BP_PartyHat.BP_PartyHat_C" (Math|Transform|MakeTransform (Transformation|GetWorldLocation (Variables|Default|GetPartyHatSpawnPoint)) "0, 0, 0" "1.000000,1.000000,1.000000") "Undefined" "MultiplyWithRoot" 0 0))
  (Transformation|AttachComponentToComponent (Variables|/Game/Blueprint/BP_PartyHat.BP_PartyHat_C|GetPartyHat _returnvalue) (Variables|Default|GetTurretMesh) "None" "KeepWorld" "KeepWorld" "KeepWorld" true))

(event EventUnlockMoreHP
  (Class|HealthComponent|IncreaseHealthandMaxHealth (Variables|Default|GetHealth) (Math|Conversions|ToFloat(Integer) (Variables|Default|GetHealthIncrease))))

(event EventRevive
  (bind _health (Variables|Default|GetHealth))
  (Audio|PlaySound2D "/Game/Assets/Audio/Mech_Mending_A.Mech_Mending_A" 1.0 1.0 0.0 0 0)
  (Utilities|FlowControl|Delay 1.5)
  (Rendering|SetActorHiddenInGame false)
  (Actor|Tick|SetActorTickEnabled true)
  (Class|HealthComponent|Heal _health (Class|HealthComponent|GetMaxHealth _health))
  (Class|Tank|ResurrectingbAlive))

(event Input|KeyboardEvents|DebugKeyP
  (params (Key :type Key%20Structure :default "None") (ActionValue :type Input%20Action%20Value%20Structure))
  (bind _basemesh (Variables|Default|GetBaseMesh))
  (bind _returnvalue (Transformation|GetWorldRotation _basemesh))
  (:Pressed
    (Niagara|SpawnSystematLocation "/Game/Assets/VFX/KTP_Effect/Particles/Fly/Others/Trail_09_07.Trail_09_07" (Transformation|GetWorldLocation _basemesh) (Math|Rotator|MakeRotator (.roll _returnvalue) (.pitch _returnvalue) (+ (.yaw _returnvalue) 9e+01)))))

(fn ConstructionScript)

(fn IsPlayer?
  (return (Class|Pawn|IsPawnControlled)))