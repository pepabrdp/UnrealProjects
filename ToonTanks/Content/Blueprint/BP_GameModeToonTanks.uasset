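; Game mode Blueprint for ToonTanks that handles the start screen, player HUD and game-over events.
; StartGame and SpawnHUD each create their widget and add it to the viewport.
; GameOver spawns a BP_Boon at the last robot's location on a win and does nothing on a loss.
; The end-game widget with win or loss text is left unconnected, so it never appears.
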(event EventBeginPlay)

(event EventTick
  (params (DeltaSeconds :type Float%20%28single-precision%29)))

(event EventStartGame
  (bind _returnvalue (UserInterface|CreateWidget "/Game/Blueprint/Widgets/WBP_StartGameWidget.WBP_StartGameWidget_C"))
  (UserInterface|Viewport|AddtoViewport _returnvalue 0))

(event EventGameOver
  (params (bWonGame :type Boolean) (LastRobotLocation :type Vector :default "0, 0, 0"))
  (if bWonGame
    (Game|SpawnActorfromClass "/Game/Blueprint/BP_Boon.BP_Boon_C" (Math|Transform|MakeTransform LastRobotLocation "0, 0, 0" "1.000000,1.000000,1.000000") "Undefined" "MultiplyWithRoot" 0 0)))

(event EventSpawnHUD
  (bind _returnvalue (UserInterface|CreateWidget "/Game/Blueprint/Widgets/WBP_HUDPlayer.WBP_HUDPlayer_C"))
  (UserInterface|Viewport|AddtoViewport _returnvalue 0))

(fn ConstructionScript)